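; Player Blueprint that registers Enhanced Input and provides a toggleable flashlight.
; BeginPlay adds the IMC_PlayerInput mapping context to player controller 0's input subsystem.
; The FlashLight action drives a FlipFlop that switches SpotLight intensity on and off and swaps a Flashlight material slot to match.
; The IA_Horizontal action only resets the Horizontal variable to zero; no movement is applied in this graph.
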(event Input|EnhancedActionEvents|EnhancedInputActionFlashLight
  (params (ActionValue :type Boolean) (ElapsedSeconds :type Float%20%28double-precision%29) (TriggeredSeconds :type Float%20%28double-precision%29) (InputAction :type Input%20Action%20Object%20Reference :default "/Game/KCY/Input/FlashLight.FlashLight"))
  (:Started
    (Utilities|FlowControl|FlipFlop
      (:A
        (Rendering|Components|Light|SetIntensity (Variables|Default|GetSpotLight) 1e+06)
        (Rendering|Material|SetMaterial (Variables|Default|Getflashlight) 1 "/Game/KCY/FlashLight/Material_002.Material_002"))
      (:B
        (Rendering|Components|Light|SetIntensity (Variables|Default|GetSpotLight) 0.0)
        (Rendering|Material|SetMaterial (Variables|Default|Getflashlight) 1 "/Game/KCY/FlashLight/Material_001.Material_001")))))

(event Input|EnhancedActionEvents|EnhancedInputActionIA_Horizontal
  (params (ActionValue :type Vector :default "0, 0, 0") (ElapsedSeconds :type Float%20%28double-precision%29) (TriggeredSeconds :type Float%20%28double-precision%29) (InputAction :type Input%20Action%20Object%20Reference :default "/Game/KCY/Input/IA_Horizontal.IA_Horizontal"))
  ;[0.15 0.15 0.15 0.5] MoveMent
  (Variables|Default|SetHorizontal 0.0))

(event EventBeginPlay
  ;[0.15 0.15 0.15 0.5] MoveMent
  (Input|AddMappingContext (PlayerController|LocalPlayerSubsystems|GetEnhancedInputLocalPlayerSubsystem (Game|GetPlayerController 0)) "/Game/KCY/Input/IMC_PlayerInput.IMC_PlayerInput" 0 "(bIgnoreAllPressedKeysUntilRelease=True,bForceImmediately=False,bNotifyUserSettings=False)"))

(event Collision|EventActorBeginOverlap
  (params (OtherActor :type Actor%20Object%20Reference)))

(event EventTick
  (params (DeltaSeconds :type Float%20%28single-precision%29)))

(fn ConstructionScript)