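; BP_Six is a controllable character that carries a flashlight and can walk, jump and crouch.
; On BeginPlay it spawns BP_Flashlight and snaps it to the mesh's Flashlight socket.
; Tick turns the move axes into normalized world-space movement with inverted vertical input, while action inputs drive jump and hold-to-crouch.
; An older WalkSpeed-scaled movement and slerped look-rotation path remains unconnected.
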(event EventBeginPlay
  (Utilities|FlowControl|Sequence
    (:then_0
      ;[0.15 0.15 0.15 0.5] 손에 손전등 붙이기
      (bind _returnvalue (Game|SpawnActorfromClass "/Game/PJW/Blueprints/BP_Flashlight.BP_Flashlight_C" (Transformation|GetSocketTransform (Variables|Character|GetMesh) "Flashlight" "RTS_World") "Undefined" "MultiplyWithRoot" 0 0))
      (Transformation|AttachComponentToComponent _returnvalue (Variables|Character|GetMesh) "Flashlight" "SnapToTarget" "SnapToTarget" "SnapToTarget" true))))

(event Collision|EventActorBeginOverlap
  (params (OtherActor :type Actor%20Object%20Reference)))

(event EventTick
  (params (DeltaSeconds :type Float%20%28single-precision%29))
  (Utilities|FlowControl|Sequence
    (:then_0
      ;[0.15 0.15 0.15 0.5] WASD 컨트롤
      (Pawn|Input|AddMovementInput (Math|Vector|Normalize (Math|Vector|MakeVector (Input|AxisValues|GetHorizontal_Move) (* (Input|AxisValues|GetVertical_Move) -1.0) 0.0)) 1.0 false))))

(event Input|ActionEvents|InputActionJump
  (params (Key :type Key%20Structure :default "None"))
  ;[0.15 0.15 0.15 0.5] 점프
  (:Pressed
    (Character|Jump)))

(event Input|ActionEvents|InputActionCrouch
  (params (Key :type Key%20Structure :default "None"))
  ;[0.15 0.15 0.15 0.5] 쭈그리기
  (:Pressed
    (Character|Crouch))
  (:Released
    (Character|UnCrouch)))

(fn ConstructionScript)