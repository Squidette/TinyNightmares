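; BP_MovingCamera is a camera actor that follows the BP_Six player along spline rails.
; On BeginPlay it caches the player pawn and SetCurrentSpline picks Spline1 or Spline2 from the game mode's GameProgress.
; Each tick it eases toward the point on the active spline closest to the player using VInterpTo, changing only location, not rotation.
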(event Collision|EventActorBeginOverlap
  (params (OtherActor :type Actor%20Object%20Reference)))

(event EventTick
  (params (DeltaSeconds :type Float%20%28single-precision%29))
  (bind _currentspine (Variables|Default|GetCurrentSpine))
  (if (Utilities|IsValid _currentspine)
    (Transformation|SetActorLocation (Math|Interpolation|VInterpTo (Transformation|GetActorLocation) (Spline|FindLocationClosesttoWorldLocation _currentspine (Transformation|GetActorLocation (Variables|Default|GetPlayer)) "World") DeltaSeconds 1.2) false false)))

(event EventBeginPlay
  (Utilities|FlowControl|Sequence
    (:then_0
      (bind _asbp_six (Utilities|Casting|CastToBP_Six (Game|Player|GetPlayerPawn 0)))
      (Variables|Default|SetPlayer _asbp_six))
    (:then_1
      (CallFunction|SetCurrentSpline))))

(fn ConstructionScript)

(fn SetCurrentSpline
  (bind _asln2_game_mode_base (Utilities|Casting|CastToLN2_GameModeBase (Game|GetGameMode)))
  (switch int (Variables|/Game/PJW/Blueprints/LN2_GameModeBase.LN2_GameModeBase_C|GetGameProgress _asln2_game_mode_base)
    (:1
      (Variables|Default|SetCurrentSpine (Variables|/Game/PJW/Blueprints/BP_CameraSpline.BP_CameraSpline_C|GetSpline (Variables|Default|GetSpline1))))
    (:2
      (Variables|Default|SetCurrentSpine (Variables|/Game/PJW/Blueprints/BP_CameraSpline.BP_CameraSpline_C|GetSpline (Variables|Default|GetSpline2)))
      (Development|PrintString "camset2"))))