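; BP_FlashlightOpening is a flashlight actor that freezes mannequins caught in front of its right-vector axis.
; Every Tick it sphere-traces along that axis, starting slightly away from the actor, against two custom object types, with debug drawing on.
; A hit BP_MyMannequin_0 receives a Freeze call.
; A separate SimulatePhysics event turns on physics for the Flashlight component.
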(event Custom|SimulatePhysics
  (Physics|SetSimulatePhysics (Variables|Default|GetFlashlight) true))

(event EventBeginPlay)

(event Collision|EventActorBeginOverlap
  (params (OtherActor :type Actor%20Object%20Reference)))

(event EventTick
  (params (DeltaSeconds :type Float%20%28single-precision%29))
  (bind _returnvalue (Transformation|GetActorRightVector))
  (bind _returnvalue_2 (Transformation|GetActorLocation))
  (bind (_outhit _returnvalue_3) (Collision|SphereTraceForObjects (+ _returnvalue_2 (* _returnvalue 2e+02)) (+ _returnvalue_2 (* _returnvalue 1e+03)) 1e+02 (Utilities|Array|MakeArray "ObjectTypeQuery10" "ObjectTypeQuery9") false 0 "ForOneFrame"))
  (if _returnvalue_3
    (bind _asbp_my_mannequin_0 (Utilities|Casting|CastToBP_MyMannequin_0 (.HitActor (Collision|BreakHitResult _outhit))))
    (Default|Freeze _asbp_my_mannequin_0)))

(fn ConstructionScript)