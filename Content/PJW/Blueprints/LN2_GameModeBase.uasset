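; LN2_GameModeBase is a game mode that tracks level progress and drives changes to the moving camera.
; Each tick it compares the player pawn's X position to a hardcoded threshold for the current GameProgress stage, advancing from stage 1 to 2 to 3.
; SetGameProgress stores the new stage, finds the BP_MovingCamera actor, calls its SetCurrentSpline and prints a debug message.
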(event EventBeginPlay
  (Variables|Default|SetPlayerPawn (Game|Player|GetPlayerPawn 0)))

(event EventTick
  (params (DeltaSeconds :type Float%20%28single-precision%29))
  (bind _playerpawn (Variables|Default|GetPlayerPawn))
  (bind _returnvalue (Transformation|GetActorLocation _playerpawn))
  (switch int (Variables|Default|GetGameProgress)
    (:1
      (if (<= (.x _returnvalue) -293.0)
        (CallFunction|SetGameProgress 2)))
    (:2
      (if (<= (.x _returnvalue) -3652.0)
        (CallFunction|SetGameProgress 3)))))

(fn ConstructionScript)

(fn SetGameProgress
  (params (stage :type Integer))
  (Variables|Default|SetGameProgress stage)
  (bind _returnvalue (Actor|GetActorOfClass "/Game/PJW/Blueprints/BP_MovingCamera.BP_MovingCamera_C"))
  (Default|SetCurrentSpline _returnvalue)
  (Development|PrintString "progressSet"))